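; Game mode that runs the start, win and game-over states for a first-person game.
; BeginPlay shows a start widget, disables character input, shows the cursor and pauses.
; Tick polls the FirstPersonCharacter, showing the win widget when Score exceeds GameWinningScore, otherwise the game-over widget when Health drops below zero.
; Both outcomes pause the game, but only game over re-enables the mouse cursor.
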(event EventBeginPlay
  (bind _returnvalue (Game|GetPlayerController 0))
  (bind _returnvalue_2 (UserInterface|CreateWidget "/Game/BeginPlayWidget.BeginPlayWidget_C"))
  (UserInterface|Viewport|AddtoViewport _returnvalue_2 0)
  (Input|DisableInput (Game|GetPlayerCharacter 0) _returnvalue)
  (Variables|/Script/Engine.PlayerController|SetbShowMouseCursor _returnvalue true)
  (Game|SetGamePaused true))

(event EventTick
  (params (DeltaSeconds :type Float%20%28single-precision%29))
  (bind _asfirst_person_character (Utilities|Casting|CastToFirstPersonCharacter (Game|GetPlayerCharacter 0)))
  (if (> (Variables|/Game/FirstPersonCharacter.FirstPersonCharacter_C|GetScore _asfirst_person_character) (Variables|Default|GetGameWinningScore))
    (bind _returnvalue (UserInterface|CreateWidget "/Game/GameWinWidget.GameWinWidget_C"))
    (UserInterface|Viewport|AddtoViewport _returnvalue 0)
    (Game|SetGamePaused true)
    (elif (< (Variables|/Game/FirstPersonCharacter.FirstPersonCharacter_C|GetHealth _asfirst_person_character) 0.0)
      (bind _returnvalue_2 (UserInterface|CreateWidget "/Game/GameOverWidget.GameOverWidget_C"))
      (UserInterface|Viewport|AddtoViewport _returnvalue_2 0)
      (Game|SetGamePaused true)
      (Variables|/Script/Engine.PlayerController|SetbShowMouseCursor (Game|GetPlayerController 0) true))))

(fn ConstructionScript)